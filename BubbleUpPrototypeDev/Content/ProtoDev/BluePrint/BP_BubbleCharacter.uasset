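; Player bubble that drifts by a constant per-tick offset while Enhanced Input steers it sideways with accumulating, clamped speed and optional inversion.
; A per-tick sphere trace detects obstacles and replaces the drift with a push along the impact normal, applied as a local offset, until a one-second delay clears it.
; Events forward countdown changes, open the pause menu, and handle death or level end by showing widgets and destroying the actor.
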(event `self.ReceiveBeginPlay`
  (set `self.IsDead?` false)
  (`EnhancedInputSubsystemInterface.AddMappingContext` (pcsubsystem `EnhancedInputLocalPlayerSubsystem` (`GameplayStatics.GetPlayerController` 0)) "/Game/ThirdPerson/Input/IMC_Default.IMC_Default" 0 (struct)))

(event `EnhancedInput|/Game/ThirdPerson/Input/Actions/IA_Move`
  (params (ActionValue :type "Vector2D Structure") (ElapsedSeconds :type "Float (double-precision)") (TriggeredSeconds :type "Float (double-precision)") (InputAction :type "InputAction Object Reference" :default "/Game/ThirdPerson/Input/Actions/IA_Move.IA_Move"))
  (:`Triggered`
    (if (not (`self.IsDead?`))
      (bind _output_get (set `self.Speed` (`KismetMathLibrary.FClamp` (+ (* (`KismetMathLibrary.SelectFloat` (* ActionValue_X -1.0) ActionValue_X (`self.InvertInput?`)) (`GameplayStatics.GetWorldDeltaSeconds`) (`self.MultiplyDeltaTime`)) (`self.Speed`)) -10.0 10.0)))
      (`self.K2_AddActorLocalOffset` (`KismetMathLibrary.MakeVector` 0.0 _output_get))))
  (:`Completed`
    (set `self.Speed` 0.0)))

(event `self.ReceiveTick`
  (params (DeltaSeconds :type "Float (single-precision)"))
  (bind _returnvalue (`SceneComponent.K2_GetComponentLocation` (`self.Sphere`)))
  (`|ExecutionSequence`
    (:`then_0`
      (bind (_outhit _returnvalue_2) (`KismetSystemLibrary.SphereTraceSingleForObjects` :`Start` _returnvalue :`End` _returnvalue :`Radius` 55.0 :`ObjectTypes` (`|MakeArray` "ObjectTypeQuery7" :!type "EObjectTypeQuery Enum") :`DrawDebugType` "ForOneFrame"))
      (if _returnvalue_2
        (set `self.ImpactNormal` (`.ImpactNormal` (`GameplayStatics.BreakHitResult` _outhit)))
        (set `self.collided` true)))
    (:`then_1`
      (if (`self.collided`)
        (`self.K2_AddActorLocalOffset` (`self.ImpactNormal`))
        (`KismetSystemLibrary.Delay` 1.0)
        (set `self.collided` false)
        (else
          (`self.K2_AddActorLocalOffset` (`self.DeltaLocation`)))))))

(event `KillPlayer`
  (set `self.IsDead?` true)
  (`UserWidget.AddToViewport` (`self.GameOver`) 0)
  (`/Game/ProtoDev/UI_WP/WP_DeathCounter.AddDeath` (`self.DeathCount`))
  (`self.K2_DestroyActor`))

(event `DecreaseCountDown`
  (`/Game/ProtoDev/UI_WP/WP_Countdown.DecreaseCountdown` (`self.Countdown`)))

(event `IncreaseCountDown`
  (`/Game/ProtoDev/UI_WP/WP_Countdown.IncreaseCOuntdown` (`self.Countdown`)))

(event `EnhancedInput|/Game/ThirdPerson/Input/Actions/IA_Pause`
  (params (ActionValue :type Boolean) (ElapsedSeconds :type "Float (double-precision)") (TriggeredSeconds :type "Float (double-precision)") (InputAction :type "InputAction Object Reference" :default "/Game/ThirdPerson/Input/Actions/IA_Pause.IA_Pause"))
  (bind _returnvalue (`GameplayStatics.GetPlayerController` 0))
  (:`Started`
    (`UserWidget.AddToViewport` (`self.PauseMenu`) 0)
    (set `PlayerController.bShowMouseCursor` true _returnvalue)
    (`WidgetBlueprintLibrary.SetInputMode_UIOnlyEx` _returnvalue null)
    (`GameplayStatics.SetGamePaused` true)
    (set `/Game/ProtoDev/UI_WP/WP_Countdown.GamePaused?` true (`self.Countdown`))))

(event `EndLevel`
  (set `self.IsDead?` true)
  (`UserWidget.AddToViewport` (`self.EndLevelWidget`) 0)
  (`GameplayStatics.SetGamePaused` true)
  (set `/Game/ProtoDev/UI_WP/WP_Countdown.GamePaused?` true (`self.Countdown`))
  (`self.K2_DestroyActor`))

(fn `UserConstructionScript`)